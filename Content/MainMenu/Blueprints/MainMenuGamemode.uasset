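; Main menu game mode for an RTS that drives menu navigation and launches singleplayer maps.
; On BeginPlay it shows the main menu and applies graphics scalability from the game instance's settings.
; Events swap widgets for options, credits, quit confirmation and singleplayer screens, with some triggering camera calls.
; Free game and free build starts save start settings, show a loading screen and open levels by MapID; only map 0 is named.
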(event Custom|Beende%20Spiel
  ;[1 1 1] Beende Spiel
  (Game|QuitGame 0 "Quit"))

(event Custom|Beenden%20Fenster
  ;[1 1 1] Bestätigung zum Beenden des Spiels
  (bind _returnvalue (UserInterface|CreateWidget "/Game/MainMenu/UI/ConfirmClose.ConfirmClose_C"))
  (bind _output_get (Variables|Default|SetConfirmCloseRef _returnvalue))
  (UserInterface|Viewport|AddtoViewport _output_get 0))

(event Custom|SpielmodusAuswählenFenster
  (bind _singleplayerspielmodusref (Variables|Default|GetSingleplayerSpielmodusRef))
  ;[1 1 1] SpielmodusAuswahlEmilNeu
  (Utilities|IsValid _singleplayerspielmodusref
    (:Is%20Valid
      (Widget|RemovefromParent _singleplayerspielmodusref))
    (:Is%20Not%20Valid
      _))
  (bind _returnvalue (UserInterface|CreateWidget "/Game/RTS/UIS/EmilsNeueSpielwiese/SpielmodusAuswahl.SpielmodusAuswahl_C"))
  (bind _output_get (Variables|Default|SetSinglePlayerSpielModusAuswahlRef _returnvalue))
  (UserInterface|Viewport|AddtoViewport _output_get 0))

(event Custom|ErstelleSingleplayerFreiesSpielMenü
  (bind _hauptmenüref (Variables|Default|GetHauptmenüRef))
  ;[1 1 1] Erstellt Singleplayer freies Spiel Menü Widget
  (Utilities|IsValid _hauptmenüref
    (:Is%20Valid
      (Widget|RemovefromParent _hauptmenüref))
    (:Is%20Not%20Valid
      _))
  (bind _returnvalue (UserInterface|CreateWidget "/Game/MainMenu/UI/SingleplayerEigenesSpiel.SingleplayerEigenesSpiel_C"))
  (Variables|Default|SetSingleplayerFreiesSpielRef _returnvalue)
  (UserInterface|Viewport|AddtoViewport (Variables|Default|GetSingleplayerFreiesSpielRef) 0))

(event Custom|StartSingleplayerSpielFreiesSpiel
  (params (MapID :type Integer) (StartEinstellungenSingleplayer :type Singleplayer%20Starteinstellungen%20Struct%20Structure))
  ;[1 1 1] Starte Singleplayermodus: Freies Spiel
  (Variables|Default|SetSingleplayerStartSettingsStruct StartEinstellungenSingleplayer)
  (CallFunction|SaveStartStats)
  (Default|ShowLoadingScreen (.AsRTSGameinstance (Utilities|Casting|CastToRTSGameinstance (Game|GetGameInstance))))
  (Utilities|FlowControl|Delay 0.05)
  (switch int MapID
    (:0
      (bind _boutsuccess (Class|LevelStreamingKismet|LoadLevelInstance "ES1vs1KleinWald" "0, 0, 0" "0, 0, 0"))
      (if _boutsuccess
        (Game|OpenLevel(byName) "ES1vs1KleinWald")))
    (:1
      (bind _boutsuccess_2 (Class|LevelStreamingKismet|LoadLevelInstance "" "0, 0, 0" "0, 0, 0"))
      (if _boutsuccess_2
        (Game|OpenLevel(byName) "")))
    (:2
      (bind _boutsuccess_3 (Class|LevelStreamingKismet|LoadLevelInstance "" "0, 0, 0" "0, 0, 0"))
      (if _boutsuccess_3
        (Game|OpenLevel(byName) "")))))

(event Custom|ErstelleSingleplayerSpielLaden
  (bind _singleplayerspielmodusref (Variables|Default|GetSingleplayerSpielmodusRef))
  (Utilities|IsValid _singleplayerspielmodusref
    (:Is%20Valid
      (Widget|RemovefromParent _singleplayerspielmodusref))
    (:Is%20Not%20Valid
      _))
  (bind _returnvalue (UserInterface|CreateWidget "/Game/MainMenu/UI/SingleplayerSpielLaden.SingleplayerSpielLaden_C"))
  (bind _output_get (Variables|Default|SetSingleplayerSpielLadenRef _returnvalue))
  (UserInterface|Viewport|AddtoViewport _output_get 0))

(event Custom|SzenarienAuswahl
  (bind _singleplayerspielmodusref (Variables|Default|GetSingleplayerSpielmodusRef))
  ;[1 1 1] SzenatienAuswahl
  (Utilities|IsValid _singleplayerspielmodusref
    (:Is%20Valid
      (Widget|RemovefromParent _singleplayerspielmodusref))
    (:Is%20Not%20Valid
      _))
  (bind _returnvalue (UserInterface|CreateWidget "/Game/RTS/UIS/EmilsNeueSpielwiese/SzenarienAuswahl.SzenarienAuswahl_C"))
  (bind _output_get (Variables|Default|SetSinglePlayerSenarienAuswahlRef _returnvalue))
  (UserInterface|Viewport|AddtoViewport _output_get 0))

(event Custom|ErstelleSingleplayerFreiesBauenMenü
  (bind _singleplayerspielmodusref (Variables|Default|GetSingleplayerSpielmodusRef))
  (Utilities|IsValid _singleplayerspielmodusref
    (:Is%20Valid
      (Widget|RemovefromParent _singleplayerspielmodusref))
    (:Is%20Not%20Valid
      _))
  (bind _returnvalue (UserInterface|CreateWidget "/Game/MainMenu/UI/SingleplayerFreiesBauen.SingleplayerFreiesBauen_C"))
  (bind _output_get (Variables|Default|SetSingleplayerFreiesBauenRef _returnvalue))
  (UserInterface|Viewport|AddtoViewport _output_get 0))

(event Custom|ErstelleSingleplayerModusMenü
  (bind _hauptmenüref (Variables|Default|GetHauptmenüRef))
  (Utilities|IsValid _hauptmenüref
    (:Is%20Valid
      (Widget|RemovefromParent _hauptmenüref))
    (:Is%20Not%20Valid
      _))
  (bind _returnvalue (UserInterface|CreateWidget "/Game/MainMenu/UI/SingleplayerSpielmodus.SingleplayerSpielmodus_C"))
  (bind _output_get (Variables|Default|SetSingleplayerSpielmodusRef _returnvalue))
  (UserInterface|Viewport|AddtoViewport _output_get 0))

(event Custom|StartSingleplayerSpielFreiesBauen
  (params (MapID :type Integer))
  (CallFunction|SaveStartStats)
  (Default|ShowLoadingScreen (.AsRTSGameinstance (Utilities|Casting|CastToRTSGameinstance (Game|GetGameInstance))))
  (Utilities|FlowControl|Delay 0.05)
  (switch int MapID
    (:0
      (bind _boutsuccess (Class|LevelStreamingKismet|LoadLevelInstance "FB1vs1KleinWald" "0, 0, 0" "0, 0, 0"))
      (if _boutsuccess
        (Game|OpenLevel(byName) "FB1vs1KleinWald")))
    (:1
      (bind _boutsuccess_2 (Class|LevelStreamingKismet|LoadLevelInstance "" "0, 0, 0" "0, 0, 0"))
      (if _boutsuccess_2
        (Game|OpenLevel(byName) "")))
    (:2
      (bind _boutsuccess_3 (Class|LevelStreamingKismet|LoadLevelInstance "" "0, 0, 0" "0, 0, 0"))
      (if _boutsuccess_3
        (Game|OpenLevel(byName) "")))))

(event Custom|ErstelleCreditsMenü
  (Utilities|IsValid (Variables|Default|GetConfirmCloseRef)
    (:Is%20Valid
      (Widget|RemovefromParent (Variables|Default|GetConfirmCloseRef)))
    (:Is%20Not%20Valid
      _))
  (Widget|RemovefromParent (Variables|Default|GetHauptmenüRef))
  (bind _returnvalue (UserInterface|CreateWidget "/Game/MainMenu/UI/Credits.Credits_C"))
  (bind _output_get (Variables|Default|SetCreditsmenüRef _returnvalue))
  (UserInterface|Viewport|AddtoViewport _output_get 0))

(event Custom|ErstelleHauptmenü
  ;[1 1 1] Hauptmenü erstellen
  (bind _returnvalue (UserInterface|CreateWidget "/Game/MainMenu/UI/MainMenu.MainMenu_C"))
  (bind _output_get (Variables|Default|SetHauptmenüRef _returnvalue))
  (UserInterface|Viewport|AddtoViewport _output_get 0)
  (Input|SetInputModeUIOnly (Game|GetPlayerController 0) (Variables|Default|GetHauptmenüRef) "DoNotLock")
  (Variables|/Script/Engine.PlayerController|SetbShowMouseCursor (Game|GetPlayerController 0) true)
  (Default|CallIntroKamera))

(event Custom|SpielerAuswahLStarten
  (params (MAPID :type Integer))
  (bind _singleplayerspielmodusref (Variables|Default|GetSingleplayerSpielmodusRef))
  ;[1 1 1] NationenAuswahl
  (Utilities|IsValid _singleplayerspielmodusref
    (:Is%20Valid
      (Widget|RemovefromParent _singleplayerspielmodusref))
    (:Is%20Not%20Valid
      _))
  (bind _returnvalue (UserInterface|CreateWidget "/Game/RTS/UIS/EmilsNeueSpielwiese/Spielerauswahl.Spielerauswahl_C" 0 MAPID))
  (bind _output_get (Variables|Default|SetSinglePlayerSpielerAuswahlRef _returnvalue))
  (UserInterface|Viewport|AddtoViewport _output_get 0))

(event Custom|BeendenFensterBeenden
  ;[1 1 1] BeendetDasBeendenFenser
  (Widget|RemovefromParent (Variables|Default|GetConfirmCloseRef)))

(event Custom|VomEinstellungsmenüZurück
  (Widget|RemovefromParent (Variables|Default|GetOptionsmenüRef))
  (Utilities|IsValid (Variables|Default|GetHauptmenüRef)
    (:Is%20Valid
      (UserInterface|Viewport|AddtoViewport (Variables|Default|GetHauptmenüRef) 0))
    (:Is%20Not%20Valid
      (bind _returnvalue (UserInterface|CreateWidget "/Game/MainMenu/UI/MainMenu.MainMenu_C"))
      (bind _output_get (Variables|Default|SetHauptmenüRef _returnvalue))
      (UserInterface|Viewport|AddtoViewport _output_get 0)
      (Default|CallEinstellungenKamera true))))

(event Custom|ErstelleOptionsmenü
  ;[1 1 1] Optionsmenü erstellen
  (Utilities|IsValid (Variables|Default|GetConfirmCloseRef)
    (:Is%20Valid
      (Widget|RemovefromParent (Variables|Default|GetConfirmCloseRef)))
    (:Is%20Not%20Valid
      _))
  (Widget|RemovefromParent (Variables|Default|GetHauptmenüRef))
  (bind _returnvalue (UserInterface|CreateWidget "/Game/MainMenu/UI/Settings.Settings_C"))
  (bind _output_get (Variables|Default|SetOptionsmenüRef _returnvalue))
  (UserInterface|Viewport|AddtoViewport _output_get 0)
  (Default|CallEinstellungenKamera false))

(event Custom|ErstelleSingleplayerKampagneMenü
  (bind _singleplayerspielmodusref (Variables|Default|GetSingleplayerSpielmodusRef))
  (Utilities|IsValid _singleplayerspielmodusref
    (:Is%20Valid
      (Widget|RemovefromParent _singleplayerspielmodusref))
    (:Is%20Not%20Valid
      _))
  (bind _returnvalue (UserInterface|CreateWidget "/Game/MainMenu/UI/SingleplayerKampange.SingleplayerKampange_C"))
  (bind _output_get (Variables|Default|SetSingleplayerKampagneRef _returnvalue))
  (UserInterface|Viewport|AddtoViewport _output_get 0))

(event EventBeginPlay
  (bind _asrtsgameinstance (Utilities|Casting|CastToRTSGameinstance (Game|GetGameInstance)))
  (Default|DoesSettingsSaveExist? _asrtsgameinstance)
  (CallFunction|ErstelleHauptmenü)
  (Variables|Default|SetSettings (Variables|/Game/Multiplayer/AllLevels/RTSGameinstance.RTSGameinstance_C|GetSettingsStruct _asrtsgameinstance))
  (bind _returnvalue (Settings|GetGameUserSettings))
  (switch string (.Grafikeinstellungen (Utilities|Struct|BreakSettingsStruct (Variables|/Game/Multiplayer/AllLevels/RTSGameinstance.RTSGameinstance_C|GetSettingsStruct _asrtsgameinstance)))
    (:Niedrig
      (Class|GameUserSettings|SetOverallScalabilityLevel _returnvalue))
    (:Mittel
      (Class|GameUserSettings|SetOverallScalabilityLevel _returnvalue 1))
    (:Hoch
      (Class|GameUserSettings|SetOverallScalabilityLevel _returnvalue 2))
    (:Episch
      (Class|GameUserSettings|SetOverallScalabilityLevel _returnvalue 3)))
  (Class|GameUserSettings|ApplySettings _returnvalue true)
  (Variables|Default|SetGrafikeinstellungen (.Grafikeinstellungen (Utilities|Struct|BreakSettingsStruct (Variables|/Game/Multiplayer/AllLevels/RTSGameinstance.RTSGameinstance_C|GetSettingsStruct _asrtsgameinstance))))
  (Variables|Default|SetSpiellautstärke (.Lautstärke (Utilities|Struct|BreakSettingsStruct (Variables|/Game/Multiplayer/AllLevels/RTSGameinstance.RTSGameinstance_C|GetSettingsStruct _asrtsgameinstance)))))

(event EventTick
  (params (DeltaSeconds :type Float%20%28single-precision%29)))

(fn ConstructionScript)

(fn SaveStartStats
  (Utilities|IsValid (Variables|Default|GetSinglePlayerStartSettingsSave)
    (:Is%20Valid
      _)
    (:Is%20Not%20Valid
      (bind _returnvalue (SaveGame|CreateSaveGameObject "/Game/MainMenu/Blueprints/SingleplayerStartEinstellungenSave.SingleplayerStartEinstellungenSave_C"))
      (Variables|Default|SetSinglePlayerStartSettingsSave _returnvalue)))
  (Variables|/Game/MainMenu/Blueprints/SingleplayerStartEinstellungenSave.SingleplayerStartEinstellungenSave_C|SetS_SingleplayerStartSettingsSave (Variables|Default|GetSinglePlayerStartSettingsSave) (Variables|Default|GetSingleplayerStartSettingsStruct))
  (SaveGame|SaveGametoSlot (Variables|Default|GetSinglePlayerStartSettingsSave) (Variables|Default|GetSaveGameSlotNameSingleplayer)))

(fn LoadStartStats
  (bind _returnvalue (SaveGame|LoadGamefromSlot (Variables|Default|GetSaveGameSlotNameSingleplayer)))
  (bind _assingleplayer_start_einstellungen_save (Utilities|Casting|CastToSingleplayerStartEinstellungenSave _returnvalue))
  (Variables|Default|SetSinglePlayerStartSettingsSave _assingleplayer_start_einstellungen_save)
  (Variables|Default|SetSingleplayerStartSettingsStruct (Variables|/Game/MainMenu/Blueprints/SingleplayerStartEinstellungenSave.SingleplayerStartEinstellungenSave_C|GetS_SingleplayerStartSettingsSave _assingleplayer_start_einstellungen_save)))

(fn SaveGameCheckStartStats
  (bind _returnvalue (SaveGame|DoesSaveGameExist (Variables|Default|GetSaveGameSlotNameSingleplayer)))
  (if _returnvalue
    (CallFunction|LoadStartStats)
    (else
      (CallFunction|SaveStartStats)
      (CallFunction|LoadStartStats))))