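; Placement ghost for RTS buildings, previewing a structure with meshes from GebäudeStruct.
; Overlapping a GebäudeActor swaps in the red mesh and sets BadTerrain on the free-build controller; any end overlap resets both.
; ErmittlePlayerController stores that controller only for singleplayer game mode 2, so otherwise only the mesh feedback applies.
; The money check is unconnected and never runs.
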(event EventBeginPlay
  (Components|StaticMesh|SetStaticMesh (Variables|Debug|GetStaticMeshComponent) (.GhostActor (Utilities|Struct|BreakGebäudeDatenBankStruktur (Variables|Default|GetGebäudeStruct))))
  (Utilities|ErmittlePlayerController))

(event EventTick
  (params (DeltaSeconds :type Float%20%28single-precision%29)))

(event Collision|EventActorBeginOverlap
  (params (OtherActor :type Actor%20Object%20Reference))
  (bind _freiesbauenpcref (Variables|Default|GetFreiesBauenPCRef))
  (if (== (Utilities|GetClass OtherActor) "/Game/RTS/Blueprints/BuildingBlueprints/GebäudeActor.GebäudeActor_C")
    (Components|StaticMesh|SetStaticMesh (Variables|Debug|GetStaticMeshComponent) (.OverlappingRed (Utilities|Struct|BreakGebäudeDatenBankStruktur (Variables|Default|GetGebäudeStruct))))
    (Utilities|IsValid _freiesbauenpcref
      (:Is%20Valid
        (Variables|/Game/Singleplayer/FreiesBauen/Blueprints/FreiesBauenPC.FreiesBauenPC_C|SetBadTerrain _freiesbauenpcref true)))))

(event Collision|EventActorEndOverlap
  (params (OtherActor :type Actor%20Object%20Reference))
  (bind _freiesbauenpcref (Variables|Default|GetFreiesBauenPCRef))
  (Components|StaticMesh|SetStaticMesh (Variables|Debug|GetStaticMeshComponent) (.GhostActor (Utilities|Struct|BreakGebäudeDatenBankStruktur (Variables|Default|GetGebäudeStruct))))
  (Utilities|IsValid _freiesbauenpcref
    (:Is%20Valid
      (Variables|/Game/Singleplayer/FreiesBauen/Blueprints/FreiesBauenPC.FreiesBauenPC_C|SetBadTerrain _freiesbauenpcref false))))

(fn ConstructionScript)