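; RTS selection square actor (AuswahlQuadrat) that sizes a box collision to span from the actor to a given world point.
; ReDrawArea converts that point to local space and halves it, using the result as the box's center and its absolute X/Y as extents.
; BeginPlay caches the RTSCameraController as Commander.
; Overlap handling is empty, and the code moving and scaling the visual area is disconnected.
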(event EventBeginPlay
  (bind _asrtscamera_controller (Utilities|Casting|CastToRTSCameraController (Game|GetPlayerController 0)))
  (Variables|Default|SetCommander _asrtscamera_controller))

(event Collision|EventActorBeginOverlap
  (params (OtherActor :type Actor%20Object%20Reference)))

(event EventTick
  (params (DeltaSeconds :type Float%20%28single-precision%29)))

(fn ConstructionScript)

(fn ReDrawArea
  (params (AreaPosition :type Vector))
  (Variables|Default|SetPosition (Math|Transform|InverseTransformLocation (Transformation|GetWorldTransform (Variables|Default|GetScene)) AreaPosition))
  (Variables|Default|SetPosition (/ (Variables|Default|GetPosition) 2.0))
  (Components|Box|SetBoxExtent (Variables|Default|GetBox) (Math|Vector|MakeVector (Math|Float|Absolute(Float) (.X (Math|Vector|BreakVector (Variables|Default|GetPosition)))) (Math|Float|Absolute(Float) (.Y (Math|Vector|BreakVector (Variables|Default|GetPosition)))) 1.0) true)
  (Transformation|SetRelativeLocation (Variables|Default|GetBox) (Variables|Default|GetPosition) false false))