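; Troop blueprint for singleplayer free-build mode that initialises a unit's stats by name and holds military boosts per army type.
; TruppenSpawnen copies a TruppenDatenbank row into variables, then adds the matching MilitärBoosts values through Werte+Boosts.
; MilitärBoostsActivated maps a boost to its stat via TruppenWertPrüfen, but only ranged, anti-cavalry and cavalry branches write the struct.
; Despite the name, TruppenSpawnen spawns nothing, as all SpawnActor calls are disconnected.
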(event EventBeginPlay)

(event Collision|EventActorBeginOverlap
  (params (OtherActor :type Actor%20Object%20Reference)))

(event EventTick
  (params (DeltaSeconds :type Float%20%28single-precision%29)))

(fn ConstructionScript)

(fn TruppenSpawnen
  (params (Name :type String))
  (bind _militärboosts (Variables|Default|GetMilitärBoosts))
  (bind (_fernhp _ferndmg _fernreichw _infhp _infdmg _schildhp _schilddmg _antikavhp _antikavdmg _kavdmg _kavhp _kavspeed _flughp _flugdmg _xp) (Utilities|Struct|BreakTruppenBoostsNew _militärboosts))
  (bind _returnvalue (Utilities|GetDataTableRow "/Game/RTS/Datenbank/TruppenDatenbank.TruppenDatenbank" (Utilities|String|StringToName Name))
    (:then
      (Variables|Default|SetHP (.HP (Utilities|Struct|BreakArmeeProfil _returnvalue)))
      (Variables|Default|SetDmg (.DM (Utilities|Struct|BreakArmeeProfil _returnvalue)))
      (Variables|Default|SetReichweite (.Reichweite (Utilities|Struct|BreakArmeeProfil _returnvalue)))
      (Variables|Default|SetAngriffsgeschwindigkeit (.AngriffsGeschwindigkeit (Utilities|Struct|BreakArmeeProfil _returnvalue)))
      (Variables|Default|SetGeschwindigkeit (.Geschwindigkeit (Utilities|Struct|BreakArmeeProfil _returnvalue)))
      (Variables|Default|SetArmeTyp (.ArmeeTyp (Utilities|Struct|BreakArmeeProfil _returnvalue)))
      (Variables|Default|SetUpgradeStufe (.UpgradeStufe (Utilities|Struct|BreakArmeeProfil _returnvalue)))
      (Variables|Default|SetSpecial (.Special (Utilities|Struct|BreakArmeeProfil _returnvalue)))
      (Variables|Default|Setskeletalmesh (.SkeletalMesh (Utilities|Struct|BreakArmeeProfil _returnvalue)))
      (Variables|Default|SetUnterhalt+ (.Unterhalt (Utilities|Struct|BreakArmeeProfil _returnvalue)))
      (Variables|Default|SetExperience _xp)
      (switch Utilities|FlowControl|Switch|SwitchonEinheitenTypen (.ArmeeTyp (Utilities|Struct|BreakArmeeProfil _returnvalue))
        (:NewEnumerator0
          (Utilities|Werte+Boosts _fernhp _ferndmg _fernreichw))
        (:NewEnumerator1
          (Utilities|Werte+Boosts _antikavhp _antikavdmg))
        (:NewEnumerator2
          (Utilities|Werte+Boosts _kavdmg _kavhp 0 _kavspeed))
        (:NewEnumerator3
          (Utilities|Werte+Boosts _schildhp _schilddmg))
        (:NewEnumerator4
          (Utilities|Werte+Boosts _infhp _infdmg))
        (:NewEnumerator5
          (Utilities|Werte+Boosts _flughp _flugdmg))))))

(fn MilitärBoostsActivated
  (params (Truppenwert :type Truppenwerte%20Enum :default "NewEnumerator7") (Boost :type Integer) (Einheitentyp :type EinheitenTypen%20Enum :default "NewEnumerator6"))
  (switch Utilities|FlowControl|Switch|SwitchonEinheitenTypen Einheitentyp
    (:NewEnumerator0
      (bind (_hp _dmg _range) (CallFunction|TruppenWertPrüfen Boost Truppenwert))
      (Utilities|Struct|SetmembersinTruppenBoostsNew (Variables|Default|GetMilitärBoosts) _hp _dmg _range (stale _hp_5) (stale _dmg_5) (stale _hp_4) (stale _dmg_4) (stale _hp_2) (stale _dmg_2) (stale _dmg_3) (stale _hp_3) (stale _speed) (stale _hp_6) (stale _dmg_6) :!label _label))
    (:NewEnumerator1
      (bind (_hp_2 _dmg_2) (CallFunction|TruppenWertPrüfen Boost Truppenwert))
      (goto _label))
    (:NewEnumerator2
      (bind (_hp_3 _dmg_3 _range_2 _speed) (CallFunction|TruppenWertPrüfen Boost Truppenwert))
      (goto _label))
    (:NewEnumerator3
      (bind (_hp_4 _dmg_4) (CallFunction|TruppenWertPrüfen Boost Truppenwert)))
    (:NewEnumerator4
      (bind (_hp_5 _dmg_5) (CallFunction|TruppenWertPrüfen Boost Truppenwert)))
    (:NewEnumerator5
      (bind (_hp_6 _dmg_6) (CallFunction|TruppenWertPrüfen Boost Truppenwert)))))

(fn TruppenWertPrüfen
  (params (NewParam1 :type Integer) (NewParam :type Truppenwerte%20Enum :default "NewEnumerator7"))
  (switch Utilities|FlowControl|Switch|SwitchonTruppenwerte NewParam
    (:NewEnumerator0
      (return NewParam1 0 0 0))
    (:NewEnumerator1
      (return 0 NewParam1 0 0))
    (:NewEnumerator2
      (return 0 0 NewParam1 0))
    (:NewEnumerator4
      (return 0 0 0 NewParam1))))