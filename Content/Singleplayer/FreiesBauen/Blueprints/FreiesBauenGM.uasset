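; Game mode for the singleplayer free-building mode (FreiesBauen) that creates the main UI and runs the day clock.
; Tick advances a normalized Clockwork value by delta time over TimeUnit, and each whole-number rollover increments Day and fires GetDay.
; UI events change TimeUnit or pause the clock through TimeStop.
; The NPC spawn point event is an empty stub, and its actor lookup is unconnected.
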(event Custom|CreateMainUIWidget
  (bind _returnvalue (UserInterface|CreateWidget "/Game/Singleplayer/FreiesBauen/UIs/FBMainUI.FBMainUI_C"))
  (bind _output_get (Variables|Default|SetMainUIRef _returnvalue))
  (UserInterface|Viewport|AddtoViewport _output_get 0)
  (EventDispatchers|BindEventtoChangeTimeSpeed (Variables|Default|GetMainUIRef) (EventDispatchers|CreateEvent :!event Custom|ChangeTimeSpeed))
  (EventDispatchers|BindEventtoTimeStop (Variables|Default|GetMainUIRef) (EventDispatchers|CreateEvent :!event Custom|StopTime)))

(event Custom|GibSpawnpunktNPCs)

(event Custom|ChangeTimeSpeed
  (params (Value :type Integer))
  (bind _output_get (Variables|Default|SetTimeUnit (Math|Conversions|ToFloat(Integer) Value)))
  (Development|PrintString (Utilities|String|ToString(Float) _output_get)))

(event Custom|StopTime
  (params (Value :type Boolean))
  (Variables|Default|SetTimeStop Value)
  (Development|PrintString "Stop" true true "(R=1.000000,G=0.000000,B=0.000000,A=1.000000)"))

(event EventBeginPlay
  (CallFunction|CreateMainUIWidget)
  (Input|SetInputModeGameandUI (Game|GetPlayerController 0) (Variables|Default|GetMainUIRef) "DoNotLock" false))

(event EventTick
  (params (DeltaSeconds :type Float%20%28single-precision%29))
  (bind (_clockwork _daytick) (CallFunction|SetClockwork DeltaSeconds))
  (if (not (Variables|Default|GetTimeStop))
    (Variables|Default|SetClockwork _clockwork)
    (bind _output_get (Variables|Default|SetDayTick _daytick))
    (if (== _output_get 1)
      (bind _output_get_2 (Variables|Default|SetDay (+ (Variables|Default|GetDay) 1)))
      (Default|CallGetDay _output_get_2))))

(fn ConstructionScript)

(fn SetClockwork
  (params (DeltaSeconds :type Float%20%28single-precision%29))
  (bind _timeunit (Variables|Default|GetTimeUnit))
  (bind _clockwork (Variables|Default|GetClockwork))
  (bind _returnvalue (/ DeltaSeconds _timeunit))
  (bind _returnvalue_2 (+ _returnvalue _clockwork))
  (bind (_remainder _returnvalue_3) (Math|Float|Division(WholeandRemainder) _returnvalue_2 1.0))
  (return _remainder _returnvalue_3))