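; Multiplayer in-game GameMode for an RTS that manages player arrival, camera pawn spawning and session exit.
; On controller swap it records the new controller and calls ErstelleUI (create UI) on every stored controller.
; RespawnPlayer, on authority only, replaces the player's pawn with a possessed CameraPawn at a random PlayerStart.
; On logout it passes the exiting controller to RTSGameinstance's DestroySessionCaller.
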(event Custom|RespawnPlayer
  (params (Player :type Player%20Controller%20Object%20Reference))
  (bind _returnvalue (Pawn|GetControlledPawn Player))
  (Networking|SwitchHasAuthority
    (:Authority
      (bind _outactors (Actor|GetAllActorsOfClass "/Script/Engine.PlayerStart"))
      (Variables|Default|SetAllSpawnPoints _outactors)
      (Utilities|IsValid _returnvalue
        (:Is%20Valid
          (Actor|DestroyActor _returnvalue))
        (:Is%20Not%20Valid
          _))
      (bind _returnvalue_2 (Game|SpawnActorfromClass "/Game/RTS/Blueprints/CameraPawn.CameraPawn_C" (Transformation|GetActorTransform (Utilities|Array|Get(acopy) (Variables|Default|GetAllSpawnPoints) (Math|Random|RandomIntegerinRange 0 (- (Utilities|Array|Length (Variables|Default|GetAllSpawnPoints)) 1)))) "Undefined" 0 0))
      (Pawn|Possess Player _returnvalue_2))))

(event EventBeginPlay)

(event EventTick
  (params (DeltaSeconds :type Float%20%28single-precision%29)))

(event EventOnLogout
  (params (ExitingController :type Controller%20Object%20Reference))
  (bind _asmp_in_game_pc (Utilities|Casting|CastToMP_InGamePC ExitingController))
  (bind _asrtsgameinstance (Utilities|Casting|CastToRTSGameinstance (Game|GetGameInstance)))
  (Default|DestroySessionCaller _asrtsgameinstance _asmp_in_game_pc))

(event EventOnSwapPlayerControllers
  (params (OldPC :type Player%20Controller%20Object%20Reference) (NewPC :type Player%20Controller%20Object%20Reference))
  (Utilities|Array|Add (Variables|Default|GetPlayerControllers) NewPC)
  (for _array_element (Variables|Default|GetPlayerControllers)
    (bind _asmp_in_game_pc (Utilities|Casting|CastToMP_InGamePC _array_element))
    (Default|ErstelleUI _asmp_in_game_pc)))

(fn ConstructionScript)