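; MP_InGamePC is the multiplayer in-game player controller that handles player chat.
; ErstelleUI creates the IngameChat widget, adds it to the viewport and focuses it in game-and-UI input mode.
; GetChatMessage pairs the text with the name and avatar from PlayerInfo, then relays it to every controller in MP_InGameGM's PlayerControllers list.
; Each receiving controller's UpdateChat passes the message to its widget's ChatWindow.
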(event Custom|ErstelleUI
  (bind _self self)
  (bind _returnvalue (UserInterface|CreateWidget "/Game/Multiplayer/IngameChat.IngameChat_C" _self))
  (Variables|Default|SetIngameChatRef _returnvalue)
  (UserInterface|Viewport|AddtoViewport _returnvalue 0)
  (Input|SetInputModeGameandUI _self _returnvalue "DoNotLock" true))

(event Custom|GetChatMessage
  (params (TextToSend :type Text))
  (bind _playerinfo (Variables|Default|GetPlayerInfo))
  (bind (_playername _playeravatar) (Utilities|Struct|BreakPlayerInfo _playerinfo))
  (Variables|Default|SetText TextToSend)
  (Variables|Default|SetSenderName _playername)
  (Variables|Default|SetPlayerAvatar _playeravatar)
  (bind _asmp_in_game_gm (Utilities|Casting|CastToMP_InGameGM (Game|GetGameMode)))
  (for _array_element (Variables|/Game/Multiplayer/InGame/Blueprints/MP_InGameGM.MP_InGameGM_C|GetPlayerControllers _asmp_in_game_gm)
    (bind _asmp_in_game_pc (Utilities|Casting|CastToMP_InGamePC _array_element))
    (CallFunction|UpdateChat _asmp_in_game_pc (Variables|Default|GetSenderName) (Variables|Default|GetText) (Variables|Default|GetPlayerAvatar))))

(event Custom|UpdateChat
  (params (SenderName :type Text) (SenderText :type Text) (PlayerAvatar :type Texture%202D%20Object%20Reference))
  (Default|UpdateChatWindow (Variables|/Game/Multiplayer/IngameChat.IngameChat_C|GetChatWindow (Variables|Default|GetIngameChatRef)) SenderName SenderText PlayerAvatar))

(event EventBeginPlay)

(event EventTick
  (params (DeltaSeconds :type Float%20%28single-precision%29)))

(fn ConstructionScript)